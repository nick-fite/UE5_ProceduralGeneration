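; Player Blueprint that lets the player edit voxel terrain with the left mouse button.
; On press, a short Visibility line trace runs from the camera along its view direction and casts the hit actor to Chunk.
; The chunk converts the hit location to a block position for ModifyVoxel, with debug prints along the way.
; Unconnected multi-trace and normal-offset nodes remain unused.
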(event `Key|LeftMouseButton`
  (params (Key :type "Key Structure"))
  (bind _returnvalue (`GameplayStatics.GetPlayerCameraManager` 0))
  (bind _returnvalue_2 (`PlayerCameraManager.GetCameraLocation` _returnvalue))
  (:`Pressed`
    (bind (_outhit _returnvalue_3) (`KismetSystemLibrary.LineTraceSingle` _returnvalue_2 (+ (* (`KismetMathLibrary.GetForwardVector` (`PlayerCameraManager.GetCameraRotation` _returnvalue)) (300.0 300.0 300.0)) _returnvalue_2) "TraceTypeQuery1"))
    (if _returnvalue_3
      (bind (_bblockinghit _binitialoverlap _time _distance _location _impactpoint _normal _impactnormal _physmat _hitactor) (`GameplayStatics.BreakHitResult` _outhit))
      (bind _aschunk (cast `Chunk` _hitactor)
        (:`then`
          _)
        (:`CastFailed`
          (`KismetSystemLibrary.PrintString` (`KismetSystemLibrary.GetDisplayName` _aschunk))))
      (bind _returnvalue_4 (`Chunk.GetBlockPos` _aschunk _location))
      (`Chunk.ModifyVoxel` _aschunk _returnvalue_4)
      (`KismetSystemLibrary.PrintString` (`KismetStringLibrary.Conv_IntVectorToString` _returnvalue_4))))
  (:`Released`
    (`KismetSystemLibrary.PrintString` "release")))

(fn `UserConstructionScript`)